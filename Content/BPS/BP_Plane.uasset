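; BP_Plane is a physics-driven, player-controlled plane that can fire rockets.
; Mouse look applies mass-scaled pitch and roll torque to the SMP38Body component.
; Move input applies yaw torque on X and forward force on Y, adding upward force whenever the event fires.
; Pressing IA_F spawns a BP_Rocket at the Arrow component's transform, with the plane as owner and instigator.
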(event `self.ReceiveBeginPlay`)

(event `EnhancedInput|/Game/Input/Actions/IA_MouseLook`
  (params (ActionValue :type "Vector2D Structure") (ElapsedSeconds :type "Float (double-precision)") (TriggeredSeconds :type "Float (double-precision)") (InputAction :type "InputAction Object Reference" :default "/Game/Input/Actions/IA_MouseLook.IA_MouseLook"))
  (bind _sm_p38_body (`self.SM_P38_Body`))
  (bind _returnvalue (* (`PrimitiveComponent.GetMass` _sm_p38_body) 100.0))
  (:`Triggered`
    (`PrimitiveComponent.AddTorqueInRadians` (`self.SM_P38_Body`) (+ (* (`SceneComponent.GetRightVector` _sm_p38_body) (* ActionValue_Y _returnvalue 10.0)) (* (`SceneComponent.GetForwardVector` _sm_p38_body) (* ActionValue_X _returnvalue 10.0) -1.0)) "None" false)))

(event `EnhancedInput|/Game/Input/Actions/IA_F`
  (params (ActionValue :type Boolean) (ElapsedSeconds :type "Float (double-precision)") (TriggeredSeconds :type "Float (double-precision)") (InputAction :type "InputAction Object Reference" :default "/Game/Input/Actions/IA_F.IA_F"))
  (:`Started`
    (`|SpawnActorFromClass` "/Game/BPS/BP_Rocket.BP_Rocket_C" (`SceneComponent.K2_GetComponentToWorld` (`self.Arrow`)) "AlwaysSpawn" "MultiplyWithRoot" self self)))

(event `EnhancedInput|/Game/Input/Actions/IA_Move`
  (params (ActionValue :type "Vector2D Structure") (ElapsedSeconds :type "Float (double-precision)") (TriggeredSeconds :type "Float (double-precision)") (InputAction :type "InputAction Object Reference" :default "/Game/Input/Actions/IA_Move.IA_Move"))
  (bind _sm_p38_body (`self.SM_P38_Body`))
  (bind _sm_p38_body_2 (`self.SM_P38_Body`))
  (bind _returnvalue (`PrimitiveComponent.GetMass` _sm_p38_body))
  (:`Triggered`
    (`PrimitiveComponent.AddTorqueInRadians` _sm_p38_body (* (`SceneComponent.GetUpVector` _sm_p38_body) (* _returnvalue 100.0 ActionValue_X)) "None" false)
    (`PrimitiveComponent.AddForce` _sm_p38_body (* (+ (* (`SceneComponent.GetForwardVector` _sm_p38_body_2) (* ActionValue_Y (* _returnvalue 5.0))) (* (`SceneComponent.GetUpVector` _sm_p38_body_2) (* _returnvalue 10.0))) 1.0) "None" true)))

(fn `UserConstructionScript`)